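; BossBP is a melee boss that trades hits with the ThirdPersonCharacter and destroys itself when its health runs out.
; Attack plays a swipe animation and briefly enables the left-hand Punch collider, which damages the player and disables their hitbox for a second.
; Its own Hitbox takes PlayerDmg when overlapped by a slashing player, flashing a hit material and printing remaining health.
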(event OnComponentBeginOverlap(punch)
  (params (OverlappedComponent :type Primitive%20Component%20Object%20Reference) (OtherActor :type Actor%20Object%20Reference) (OtherComp :type Primitive%20Component%20Object%20Reference) (OtherBodyIndex :type Integer) (bFromSweep :type Boolean) (SweepResult :type Hit%20Result%20Structure%20%28by%20ref%29))
  (bind _asthird_person_character (Utilities|Casting|CastToThirdPersonCharacter OtherActor))
  (if (Variables|Default|GetAttacking)
    (bind _asthird_person_character_2 (Utilities|Casting|CastToThirdPersonCharacter OtherActor))
    (Default|TakeDamage _asthird_person_character_2 10)
    (bind _asthird_person_character_3 (Utilities|Casting|CastToThirdPersonCharacter (Game|GetPlayerCharacter 0)))
    (Collision|SetCollisionEnabled (Variables|/Game/ThirdPersonBP/Blueprints/ThirdPersonCharacter.ThirdPersonCharacter_C|GethitboxPlayer _asthird_person_character_3) "NoCollision")
    (Utilities|FlowControl|Delay 1.0)
    (Collision|SetCollisionEnabled (Variables|/Game/ThirdPersonBP/Blueprints/ThirdPersonCharacter.ThirdPersonCharacter_C|GethitboxPlayer _asthird_person_character_3) "QueryAndPhysics")))

(event OnComponentBeginOverlap(hitbox)
  (params (OverlappedComponent :type Primitive%20Component%20Object%20Reference) (OtherActor :type Actor%20Object%20Reference) (OtherComp :type Primitive%20Component%20Object%20Reference) (OtherBodyIndex :type Integer) (bFromSweep :type Boolean) (SweepResult :type Hit%20Result%20Structure%20%28by%20ref%29))
  ;[1 1 1] Hit by Player
  (bind _asthird_person_character (Utilities|Casting|CastToThirdPersonCharacter OtherActor))
  (if (Variables|/Game/ThirdPersonBP/Blueprints/ThirdPersonCharacter.ThirdPersonCharacter_C|GetSlashing? _asthird_person_character)
    (Rendering|Material|SetMaterial (Variables|Character|GetMesh) 0 "/Game/BunnyProject/Boss/hit.hit")
    (Utilities|FlowControl|Delay 0.2)
    (Rendering|Material|SetMaterial (Variables|Character|GetMesh) 0 "/Game/BunnyProject/Boss/Mesh_and_Animation_bs/warrok_MAT.warrok_MAT")
    (bind _output_get (Variables|Default|SetHealth (- (Variables|Default|GetHealth) (Variables|/Game/ThirdPersonBP/Blueprints/ThirdPersonCharacter.ThirdPersonCharacter_C|GetPlayerDmg _asthird_person_character))))
    (Development|PrintString (Utilities|String|ToString(Integer) _output_get) true true "(R=1.000000,G=0.000000,B=0.048927,A=1.000000)")
    (if (<= _output_get 0)
      (Actor|DestroyActor))))

(event Custom|Attack
  (Collision|SetCollisionEnabled (Variables|Default|Getpunch) "QueryAndPhysics")
  (Components|Animation|PlayAnimation (Variables|Character|GetMesh) "/Game/BunnyProject/Boss/Mesh_and_Animation_bs/Animation/Orc_Swiping.Orc_Swiping" false)
  (Variables|Default|SetAttacking true)
  (Utilities|FlowControl|Delay 1.3)
  (Collision|SetCollisionEnabled (Variables|Default|Getpunch) "NoCollision")
  (Utilities|FlowControl|Delay 1.3)
  (Variables|Default|SetAttacking false)
  (Components|Animation|SetAnimationMode (Variables|Character|GetMesh) "AnimationBlueprint"))

(event EventBeginPlay
  (Collision|SetCollisionEnabled (Variables|Default|Getpunch) "NoCollision"))

(fn ConstructionScript
  (Transformation|AttachComponentToComponent (Variables|Default|Getpunch) (Variables|Character|GetMesh) "LeftHand" "KeepRelative" "KeepRelative" "KeepRelative" true))