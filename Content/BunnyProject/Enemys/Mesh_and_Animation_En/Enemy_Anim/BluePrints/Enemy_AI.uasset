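; Enemy_AI is the AI controller for Enemy_BP pawns, driving their behavior through the Enemy_BT behavior tree.
; On possessing an Enemy_BP, it stores the pawn reference and starts the tree.
; AI Perception updates for a ThirdPersonCharacter write the sensed state to the CanSeePlayer blackboard key.
; An Attack event forwards attack requests to the possessed enemy.
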(event OnTargetPerceptionUpdated(AIPerception)
  (params (Actor :type Actor%20Object%20Reference) (Stimulus :type AI%20Stimulus%20Structure))
  (Utilities|Casting|CastToThirdPersonCharacter Actor)
  (AI|Components|Blackboard|SetValueasBool (AI|GetBlackboard 0) (Utilities|Name|MakeLiteralName "CanSeePlayer") (.bSuccessfullySensed (Utilities|Struct|BreakAIStimulus Stimulus))))

(event Custom|Attack
  (Default|Attack (Variables|Default|GetEnemy)))

(event EventPossess
  (params (PossessedPawn :type Pawn%20Object%20Reference))
  (bind _asenemy_bp (Utilities|Casting|CastToEnemy_BP PossessedPawn))
  (Variables|Default|SetEnemy _asenemy_bp)
  (AI|RunBehaviorTree "/Game/BunnyProject/Enemys/Mesh_and_Animation_En/Enemy_Anim/BluePrints/Enemy_BT.Enemy_BT"))

(fn ConstructionScript)